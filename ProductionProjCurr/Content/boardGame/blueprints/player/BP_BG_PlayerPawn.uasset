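; Player pawn for the board game, whose only working logic is putting the player HUD on screen.
; BeginPlay creates a BP_PlayerUI widget for player controller 0 and adds it to the viewport; the AddUI event runs the same path.
; The scroll input event and FuncAddui are empty.
; Build-menu toggling and scroll-driven camera FOV zoom remain only as disconnected nodes that never run.
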(event `self.ReceiveBeginPlay`
  (bind _returnvalue (`|CreateWidget` "/Game/boardGame/blueprints/player/BP_PlayerUI.BP_PlayerUI_C" (`GameplayStatics.GetPlayerController` 0) :!label _label))
  (`UserWidget.AddToViewport` _returnvalue 0))

(event `AddUI`
  (goto _label))

(event `EnhancedInput|/Game/Input/Actions/IA_Scroll`
  (params (ActionValue :type "Float (double-precision)") (ElapsedSeconds :type "Float (double-precision)") (TriggeredSeconds :type "Float (double-precision)") (InputAction :type "InputAction Object Reference" :default "/Game/Input/Actions/IA_Scroll.IA_Scroll")))

(fn `func_addui`)

(fn `UserConstructionScript`)